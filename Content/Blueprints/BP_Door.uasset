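; BP_Door is a swinging door that opens on interaction and closes automatically when the player leaves its Box trigger.
; InteractwithObject reverses a shared Timeline from its end to open the door, and the player's end overlap plays it from the start to close it.
; The Timeline track scales Angle to set the Door's yaw, and Audio plays when the Timeline finishes.
; An Open flag guards against repeated triggering.
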(event `self.Box.OnComponentEndOverlap`
  (params (OverlappedComponent :type "PrimitiveComponent Object Reference") (OtherActor :type "Actor Object Reference") (OtherComp :type "PrimitiveComponent Object Reference") (OtherBodyIndex :type Integer))
  (if (== OtherActor (`GameplayStatics.GetPlayerCharacter` 0))
    (if (`self.open`)
      (set `self.open` false)
      (bind (_direction _newtrack_0) (`Timeline|Timeline` :!via `PlayFromStart` :!label _label)
        (:`Update`
          (`SceneComponent.K2_SetRelativeRotation` (`self.Door`) (`KismetMathLibrary.MakeRotator` 90.0 0.0 (* _newtrack_0 (`self.Angle`))) false false))
        (:`Finished`
          (`AudioComponent.Play` (`self.Audio`) 0.0)
          (if (`self.open`)
            _))))))

(event `self.InteractWithObject`
  (if (not (`self.open`))
    (set `self.open` true)
    (goto _label :!via `ReverseFromEnd`)))

(fn `UserConstructionScript`
  (`parent.UserConstructionScript`))