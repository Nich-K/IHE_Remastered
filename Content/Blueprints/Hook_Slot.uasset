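; Hook_Slot is a slot actor that holds a hook and passes it to an empty neighboring slot when interacted with, like a sliding-piece puzzle.
; At BeginPlay, SpawnHook selects whether it spawns a Hook, a Hook_Objective or nothing.
; On interaction it searches its Neighbors for the first one without a valid hook and hands over the reference.
; CheckAfterUpdate then links the hook to its new slot and snaps it to that location.
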(event `self.ReceiveBeginPlay`
  (bind _spawnhook (`self.SpawnHook`))
  (if (== _spawnhook 1)
    (bind _returnvalue (`|SpawnActorFromClass` "/Game/Blueprints/Hook.Hook_C" (`self.GetTransform`) "Undefined" "MultiplyWithRoot" null null))
    (set `self.Hook` _returnvalue)
    (`self.CheckAfterUpdate` :!label _label)
    (elif (== _spawnhook 2)
      (bind _returnvalue_2 (`|SpawnActorFromClass` "/Game/Blueprints/Hook_Objective.Hook_Objective_C" (`self.GetTransform`) "Undefined" "MultiplyWithRoot" null null))
      (set `self.Hook` _returnvalue_2)
      (goto _label))))

(event `HookIsInteractedWith`
  (bind (_foundneighbor _neighbor) (`self.CheckForFreeNeigbors`))
  (if _foundneighbor
    (set `/Game/Blueprints/Hook_Slot.Hook` (`self.Hook`) _neighbor)
    (set `self.Hook` null)
    (`self.CheckAfterUpdate` _neighbor)))

(event `CheckAfterUpdate`
  (bind _hook (`self.Hook`))
  (set `/Game/Blueprints/Hook.Slot` self _hook)
  (`self.K2_SetActorLocation` _hook (`self.K2_GetActorLocation`) false false))

(fn `CheckForFreeNeigbors`
  (returns (FoundNeighbor :type Boolean) (Neighbor :type "/Game/Blueprints/Hook_Slot Object Reference"))
  (if (`KismetSystemLibrary.IsValid` (`self.Hook`))
    (for _array_element (`self.Neighbors`)
      (if (not (`KismetSystemLibrary.IsValid` (`/Game/Blueprints/Hook_Slot.Hook` _array_element)))
        (`KismetSystemLibrary.PrintString` "Hello")
        (return true _array_element)
        (else
          (`KismetSystemLibrary.PrintString` "no"))))
    (return false null)))

(fn `UserConstructionScript`)