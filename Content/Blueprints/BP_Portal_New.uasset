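; Portal actor that shows the view through its linked portal on a plane.
; On BeginPlay, after a short delay, it ticks in post-update work and creates a viewport-sized render target, feeding it to its plane's dynamic material and the linked portal's camera.
; Each tick, it places that camera at the player camera's pose relative to this portal, flipped in X and Y and re-expressed in the linked portal's space.
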(event `self.ReceiveBeginPlay`
  (bind (_returnvalue_x _returnvalue_y) (`KismetMathLibrary.BreakVector2D` (`WidgetLayoutLibrary.GetViewportSize`)))
  (`KismetSystemLibrary.Delay` 0.1)
  (`self.SetTickGroup` "TG_PostUpdateWork")
  (bind _returnvalue (`KismetMaterialLibrary.CreateDynamicMaterialInstance` "/Game/Materials/M_Portal.M_Portal"))
  (bind _output_get (set `self.Portal_Mat` _returnvalue))
  (`PrimitiveComponent.SetMaterial` (`self.Plane`) 0 _output_get)
  (bind _returnvalue_2 (`KismetRenderingLibrary.CreateRenderTarget2D` (`KismetMathLibrary.FTrunc` _returnvalue_x) (`KismetMathLibrary.FTrunc` _returnvalue_y) "RTF_RGBA8_SRGB"))
  (bind _output_get_2 (set `self.Portal_RT` _returnvalue_2))
  (`MaterialInstanceDynamic.SetTextureParameterValue` (`self.Portal_Mat`) "Texture" _output_get_2)
  (set `SceneCaptureComponent2D.TextureTarget` (`self.Portal_RT`) (`/Game/Blueprints/BP_Portal_New.Camera` (`self.Linked Portal`))))

(event `self.ReceiveTick`
  (params (DeltaSeconds :type "Float (single-precision)"))
  (`self.UpdateScreenCapture`))

(fn `UpdateScreenCapture`
  (bind _returnvalue (`self.GetTransform`))
  (bind _returnvalue_2 (`self.GetTransform` (`self.Linked Portal`)))
  (bind (_x _y _z) (`KismetMathLibrary.BreakRotIntoAxes` (`SceneComponent.K2_GetComponentRotation` (`PlayerCameraManager.TransformComponent` (`GameplayStatics.GetPlayerCameraManager` 0)))))
  (`SceneComponent.K2_SetWorldLocationAndRotation` (`/Game/Blueprints/BP_Portal_New.Camera` (`self.Linked Portal`)) (`KismetMathLibrary.TransformLocation` (`self.GetTransform` (`self.Linked Portal`)) (`KismetMathLibrary.InverseTransformLocation` (`KismetMathLibrary.MakeTransform` (.location (`self.GetTransform`)) (.rotation (`self.GetTransform`)) (`KismetMathLibrary.MakeVector` (* (.x (.scale (`self.GetTransform`))) -1.0) (* (.y (.scale (`self.GetTransform`))) -1.0) (.z (.scale (`self.GetTransform`))))) (`SceneComponent.K2_GetComponentLocation` (`PlayerCameraManager.TransformComponent` (`GameplayStatics.GetPlayerCameraManager` 0))))) (`KismetMathLibrary.MakeRotationFromAxes` (`KismetMathLibrary.TransformDirection` _returnvalue_2 (`KismetMathLibrary.MirrorVectorByNormal` (`KismetMathLibrary.MirrorVectorByNormal` (`KismetMathLibrary.InverseTransformDirection` _returnvalue _x) (1.0 0.0 0.0)) (0.0 1.0 0.0))) (`KismetMathLibrary.TransformDirection` _returnvalue_2 (`KismetMathLibrary.MirrorVectorByNormal` (`KismetMathLibrary.MirrorVectorByNormal` (`KismetMathLibrary.InverseTransformDirection` _returnvalue _y) (1.0 0.0 0.0)) (0.0 1.0 0.0))) (`KismetMathLibrary.TransformDirection` _returnvalue_2 (`KismetMathLibrary.MirrorVectorByNormal` (`KismetMathLibrary.MirrorVectorByNormal` (`KismetMathLibrary.InverseTransformDirection` _returnvalue _z) (1.0 0.0 0.0)) (0.0 1.0 0.0)))) false false))

(fn `UserConstructionScript`)